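; Interactive boarded-up door that must be cleared of its planks before it can open and close.
; A box overlap with the ThirdPersonCharacter enables Interact input and opens a gate for door toggling.
; While the Board counter is non-zero, each press drops the next wood piece via physics, ignores Pawn collision, decrements the counter and plays a hit sound.
; At zero, a FlipFlop plays or reverses a timeline that lerps the door's yaw.
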(event `InputAction|Interact` :consume false
  (params (Key :type "Key Structure"))
  ;[1 1 1] Open Door if close enough
  (:`Pressed`
    (if (== (`self.Board`) 0)
      (`/Engine/EditorBlueprintResources/StandardMacros.Gate` true :!label _label
        (:`Exit`
          ;[1 1 1] Open Close Anim
          (`/Engine/EditorBlueprintResources/StandardMacros.FlipFlop`
            (:`A`
              (bind (_direction _doortrack) (`Timeline|OpenClose` :!label _label_2)
                (:`Update`
                  (`SceneComponent.K2_SetRelativeRotation` (`self.Door`) (`KismetMathLibrary.MakeRotator` 0.0 0.0 (`KismetMathLibrary.Lerp` (`self.Close Angle`) (`self.Open Angle`) _doortrack)) false false))))
            (:`B`
              (goto _label_2 :!via `Reverse`)))))
      (else
        (`self.Remove Boards`)))))

(event `self.Box.OnComponentBeginOverlap`
  (params (OverlappedComponent :type "PrimitiveComponent Object Reference") (OtherActor :type "Actor Object Reference") (OtherComp :type "PrimitiveComponent Object Reference") (OtherBodyIndex :type Integer) (bFromSweep :type Boolean) (SweepResult :type "HitResult Structure (by ref)"))
  ;[1 1 1] Open Door if close enough
  (cast `/Game/ThirdPersonBP/Blueprints/ThirdPersonCharacter` OtherActor)
  (`self.EnableInput` (`GameplayStatics.GetPlayerController` 0))
  (goto _label :!via `Open`))

(event `self.Box.OnComponentEndOverlap`
  (params (OverlappedComponent :type "PrimitiveComponent Object Reference") (OtherActor :type "Actor Object Reference") (OtherComp :type "PrimitiveComponent Object Reference") (OtherBodyIndex :type Integer))
  ;[1 1 1] Open Door if close enough
  (cast `/Game/ThirdPersonBP/Blueprints/ThirdPersonCharacter` OtherActor)
  (`self.DisableInput` (`GameplayStatics.GetPlayerController` 0))
  (goto _label :!via `Close`))

(event `Remove Boards`
  (bind _wood2 (`self.Wood2`))
  (bind _wood0 (`self.Wood0`))
  (bind _wood (`self.Wood`))
  (bind _wood1 (`self.Wood1`))
  ;[1 1 1] Remove Boards From door
  (if (not (`SceneComponent.IsSimulatingPhysics` _wood0 "None"))
    (`PrimitiveComponent.SetSimulatePhysics` _wood0 true)
    (`PrimitiveComponent.SetCollisionResponseToChannel` _wood0 "ECC_Pawn" "ECR_Ignore")
    (bind _result (`/Engine/EditorBlueprintResources/StandardMacros.DecrementInt` (`self.Board`) :!label _label_3)
      (:`  `
        (set `self.Board` _result)
        (`GameplayStatics.PlaySoundAtLocation` "/Game/CryOfSlience/Board_Door/wooden_hit.wooden_hit" (`self.K2_GetActorLocation`) (struct) 1.0 1.0 0.0 null null null)))
    (elif (not (`SceneComponent.IsSimulatingPhysics` _wood "None"))
      (`PrimitiveComponent.SetSimulatePhysics` _wood true)
      (`PrimitiveComponent.SetCollisionResponseToChannel` _wood "ECC_Pawn" "ECR_Ignore")
      (goto _label_3)
      (elif (not (`SceneComponent.IsSimulatingPhysics` _wood1 "None"))
        (`PrimitiveComponent.SetSimulatePhysics` _wood1 true)
        (`PrimitiveComponent.SetCollisionResponseToChannel` _wood1 "ECC_Pawn" "ECR_Ignore")
        (goto _label_3)
        (elif (not (`SceneComponent.IsSimulatingPhysics` _wood2 "None"))
          (`PrimitiveComponent.SetSimulatePhysics` _wood2 true)
          (`PrimitiveComponent.SetCollisionResponseToChannel` _wood2 "ECC_Pawn" "ECR_Ignore")
          (goto _label_3))))))

(fn `UserConstructionScript`)