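; Door actor that swings open when Interact is pressed in range and closes by itself afterwards.
; OpenCollision toggles a gate for the third-person character, so the input only works inside that volume.
; Open and close timelines lerp the door's yaw between two angles, with Opened set once opening finishes.
; Ending any overlap with CloseCollision plays the close timeline if Opened is set, which is never reset here.
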(event `self.ReceiveBeginPlay`
  ;[1 1 1] Enable input
  (`self.EnableInput` (`GameplayStatics.GetPlayerController` 0)))

(event `InputAction|Interact`
  (params (Key :type "Key Structure"))
  ;[1 1 1] Interact
  (:`Pressed`
    (`/Engine/EditorBlueprintResources/StandardMacros.Gate` true :!label _label
      (:`Exit`
        ;[1 1 1] Door Open
        (bind (_direction _door_open) (`Timeline|Door Open` :!via `PlayFromStart`)
          (:`Update`
            (`SceneComponent.K2_SetRelativeRotation` (`self.Door`) (`KismetMathLibrary.MakeRotator` 0.0 0.0 (`KismetMathLibrary.Lerp` (`self.Door Close Angle`) (`self.Door Open Angle`) _door_open)) false false))
          (:`Finished`
            (set `self.Opened?` true)))))))

(event `self.Open Collision.OnComponentBeginOverlap`
  (params (OverlappedComponent :type "PrimitiveComponent Object Reference") (OtherActor :type "Actor Object Reference") (OtherComp :type "PrimitiveComponent Object Reference") (OtherBodyIndex :type Integer) (bFromSweep :type Boolean) (SweepResult :type "HitResult Structure (by ref)"))
  ;[1 1 1] Interact
  (cast `/Game/ThirdPersonBP/Blueprints/ThirdPersonCharacter` OtherActor)
  (goto _label :!via `Open`))

(event `self.Open Collision.OnComponentEndOverlap`
  (params (OverlappedComponent :type "PrimitiveComponent Object Reference") (OtherActor :type "Actor Object Reference") (OtherComp :type "PrimitiveComponent Object Reference") (OtherBodyIndex :type Integer))
  ;[1 1 1] Interact
  (cast `/Game/ThirdPersonBP/Blueprints/ThirdPersonCharacter` OtherActor)
  (goto _label :!via `Close`))

(event `self.Close Collision.OnComponentEndOverlap`
  (params (OverlappedComponent :type "PrimitiveComponent Object Reference") (OtherActor :type "Actor Object Reference") (OtherComp :type "PrimitiveComponent Object Reference") (OtherBodyIndex :type Integer))
  ;[1 1 1] Door Close
  (if (`self.Opened?`)
    (bind (_direction _door_close) (`Timeline|Door Close` :!via `PlayFromStart`)
      (:`Update`
        (`SceneComponent.K2_SetRelativeRotation` (`self.Door`) (`KismetMathLibrary.MakeRotator` 0.0 0.0 (`KismetMathLibrary.Lerp` (`self.Door Close Angle`) (`self.Door Open Angle`) _door_close)) false false)))))

(fn `UserConstructionScript`)