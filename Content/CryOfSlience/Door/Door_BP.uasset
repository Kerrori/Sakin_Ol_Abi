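; Interactable door Blueprint that swings open or closed when a player holding the matching key channel interacts with it.
; OnInteraction checks the player's key through HasKey, then toggles between Open and Close based on the Open flag.
; A single RotateDoor timeline drives the door's relative yaw, playing forward to open and reversing faster to close, with a separate sound for each.
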(event `/Game/CryOfSlience/Door/Interactable_Interface.OnInteraction`
  (params (Player :type "/Game/ThirdPersonBP/Blueprints/ThirdPersonCharacter Object Reference"))
  (`/Engine/EditorBlueprintResources/StandardMacros.IsValid` Player
    (:`Is Valid`
      (if (`/Game/ThirdPersonBP/Blueprints/ThirdPersonCharacter.HasKey?` Player (`self.KeyChannel`))
        (if (`self.Open?`)
          (`self.Close`)
          (else
            (`self.Open`)))))))

(event `Open`
  (set `self.Open?` true)
  (`TimelineComponent.SetPlayRate` (`self.RotateDoor`) 0.4)
  (`GameplayStatics.PlaySoundAtLocation` "/Game/CryOfSlience/Door/KeyDooropen.KeyDooropen" (`SceneComponent.K2_GetComponentLocation` (`self.Door`)) (struct) 1.0 1.0 0.0 null null null)
  (bind (_direction _doorrotation) (`Timeline|RotateDoor` :!label _label)
    (:`Update`
      (`SceneComponent.K2_SetRelativeRotation` (`self.Door`) (`KismetMathLibrary.MakeRotator` 0.0 0.0 _doorrotation) false false))))

(event `Close`
  (set `self.Open?` false)
  (`TimelineComponent.SetPlayRate` (`self.RotateDoor`) 0.9)
  (`GameplayStatics.PlaySoundAtLocation` "/Game/CryOfSlience/Door/closev2.closev2" (`SceneComponent.K2_GetComponentLocation` (`self.Door`)) (struct) 1.0 1.0 0.0 null null null)
  (goto _label :!via `Reverse`))

(fn `UserConstructionScript`)