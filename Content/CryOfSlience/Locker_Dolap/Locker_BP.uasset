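; Hiding-spot locker that lets the player get in and out with E while overlapping its Box.
; Box overlaps toggle input and a gate on E, which swings the door via a timeline and calls ToogleHide.
; ToogleHide hides the character, disables its collision and blends the view to the locker, or reverses this.
; While hidden, look input feeds clamped pitch and yaw, applied to the locker camera by a self-recalling delay loop.
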(event `Key|E`
  (params (Key :type "Key Structure"))
  ;[1 1 1] Get in/out Of Locker
  (:`Pressed`
    (`/Engine/EditorBlueprintResources/StandardMacros.Gate` true :!label _label
      (:`Exit`
        (`|ExecutionSequence`
          (:`then_0`
            (`self.Toogle Hide`)
            (`self.Move Camera`)
            (`KismetSystemLibrary.Delay` 0.2)
            (`self.EnableInput` (`GameplayStatics.GetPlayerController` 0) :!label _label_2)
            (goto _label :!via `Open`))
          (:`then_1`
            (bind (_direction _doortrack) (`Timeline|Open/ClosedoorT` :!via `PlayFromStart`)
              (:`Update`
                (`SceneComponent.K2_SetRelativeRotation` (`self.Locker_Door`) (`KismetMathLibrary.MakeRotator` 0.0 0.0 (`KismetMathLibrary.Lerp` (`self.Close Angle`) (`self.Open Angle`) _doortrack)) false false)))))))))

(event `self.Box.OnComponentBeginOverlap`
  (params (OverlappedComponent :type "PrimitiveComponent Object Reference") (OtherActor :type "Actor Object Reference") (OtherComp :type "PrimitiveComponent Object Reference") (OtherBodyIndex :type Integer) (bFromSweep :type Boolean) (SweepResult :type "HitResult Structure (by ref)"))
  ;[1 1 1] Get in/out Of Locker
  (bind _asthird_person_character (cast `/Game/ThirdPersonBP/Blueprints/ThirdPersonCharacter` OtherActor))
  (set `self.Charecter REF` _asthird_person_character)
  (goto _label_2))

(event `self.Box.OnComponentEndOverlap`
  (params (OverlappedComponent :type "PrimitiveComponent Object Reference") (OtherActor :type "Actor Object Reference") (OtherComp :type "PrimitiveComponent Object Reference") (OtherBodyIndex :type Integer))
  ;[1 1 1] Get in/out Of Locker
  (cast `/Game/ThirdPersonBP/Blueprints/ThirdPersonCharacter` OtherActor)
  (`self.DisableInput` (`GameplayStatics.GetPlayerController` 0))
  (goto _label :!via `Close`))

(event `InputAxis|LookUp`
  (params (AxisValue :type "Float (single-precision)"))
  ;[1 1 1] Move Camera
  (if (`self.IsHiding?`)
    (bind _output_get (set `self.Pitch` (`KismetMathLibrary.FClamp` (+ (`self.Pitch`) AxisValue) -40.0 20.0)))
    (else
      (`Pawn.AddControllerPitchInput` (`self.Charecter REF`) AxisValue))))

(event `Move Camera`
  ;[1 1 1] Move Camera
  (if (`self.IsHiding?`)
    (`SceneComponent.K2_SetRelativeRotation` (`self.Camera`) (`KismetMathLibrary.MakeRotator` 0.0 (* (stale `InputAxis|LookUp` _output_get) -1.0) (stale `InputAxis|Turn` _output_get)) false false)
    (`KismetSystemLibrary.Delay` 0.001)
    (`self.Move Camera`)))

(event `InputAxis|Turn`
  (params (AxisValue :type "Float (single-precision)"))
  ;[1 1 1] Move Camera
  (if (`self.IsHiding?`)
    (bind _output_get (set `self.Yaw` (`KismetMathLibrary.FClamp` (+ (`self.Yaw`) AxisValue) -60.0 60.0)))
    (else
      (`Pawn.AddControllerYawInput` (`self.Charecter REF`) AxisValue))))

(fn `Toogle Hide`
  (bind _returnvalue (`GameplayStatics.GetPlayerController` 0))
  (bind _charecter_ref (`self.Charecter REF`))
  (if (`self.IsHiding?`)
    (set `self.IsHiding?` false)
    (`self.SetActorHiddenInGame` _charecter_ref false)
    (`self.SetActorEnableCollision` _charecter_ref true)
    (`PlayerController.SetViewTargetWithBlend` _returnvalue _charecter_ref 0.8 "VTBlend_Linear" 0.0 false)
    (else
      (set `self.IsHiding?` true)
      (`self.SetActorHiddenInGame` _charecter_ref true)
      (`self.SetActorEnableCollision` _charecter_ref false)
      (`PlayerController.SetViewTargetWithBlend` _returnvalue self 0.8 "VTBlend_Linear" 0.0 false))))

(fn `UserConstructionScript`)