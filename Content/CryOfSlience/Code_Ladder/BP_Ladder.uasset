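; BP_Ladder is a procedurally built ladder actor whose height and rung spacing come from Height and CrossbarGap.
; InitLadder runs from the construction script and BeginPlay, moving LadderTop to Height and fitting both side rails by centering and Z-scaling them.
; It then clears and refills an instanced mesh component with thin crossbars at each gap below the top.
; The file contains only construction logic, with no climbing interaction.
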(event `self.ReceiveBeginPlay`
  (`self.Init Ladder`))

(event `Init Ladder`
  (bind _ism_crossbar (`self.Ism_CrossBar`))
  (bind _ladder_r (`self.Ladder_R`))
  (bind _temp_height (`self.Temp Height`))
  (bind _ladder_l (`self.Ladder_L`))
  (bind (_relativelocation_x _relativelocation_y _relativelocation_z) (`KismetMathLibrary.BreakVector` (`SceneComponent.RelativeLocation` (`self.Ladder Top`))))
  (`SceneComponent.K2_SetRelativeLocation` (`self.Ladder Top`) (`KismetMathLibrary.MakeVector` 0.0 0.0 (`self.Height`)) false false)
  (`self.Adjust Side Bar` _ladder_l _ladder_l)
  (`self.Adjust Side Bar` _ladder_r _ladder_r)
  (set `self.Temp Height` 0.0)
  (`InstancedStaticMeshComponent.ClearInstances` _ism_crossbar)
  (while (< _temp_height _relativelocation_z)
    (`InstancedStaticMeshComponent.AddInstance` _ism_crossbar (`KismetMathLibrary.MakeTransform` (`KismetMathLibrary.MakeVector` 0.0 0.0 _temp_height) (struct) (0.05 0.6 0.05)))
    (set `self.Temp Height` (+ _temp_height (`self.Crossbar Gap`)))))

(fn `UserConstructionScript`
  (`self.Init Ladder`))