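; Door Blueprint that the player kicks open on the first Interact press, then closes and reopens on later presses.
; An overlap box enables input and opens a gate for the ThirdPersonCharacter, reversing both on exit.
; The one-time kick snaps the character to a SkeletalMesh transform, plays a montage and swings the door by timeline.
; A start-closed DoOnce, reset on release, holds back a FlipFlop-driven open/close timeline during that first press.
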(event `InputAction|Interact`
  (params (Key :type "Key Structure"))
  (:`Pressed`
    (`|ExecutionSequence`
      (:`then_0`
        (`/Engine/EditorBlueprintResources/StandardMacros.DoOnce` false
          (:`Completed`
            (bind _asthird_person_character (cast `/Game/ThirdPersonBP/Blueprints/ThirdPersonCharacter` (`GameplayStatics.GetPlayerCharacter` 0)))
            (`self.K2_SetActorTransform` _asthird_person_character (`SceneComponent.K2_GetComponentToWorld` (`self.SkeletalMesh`)) false false)
            (`Character.PlayAnimMontage` _asthird_person_character "/Game/CryOfSlience/MixAnimations/Anim/GercekBu_Montage.GercekBu_Montage" 1.0 "None")
            (bind (_direction _door_kick_track) (`Timeline|Kick Open Door`)
              (:`Update`
                (`SceneComponent.K2_SetRelativeRotation` (`self.Door`) (`KismetMathLibrary.MakeRotator` 0.0 0.0 (`KismetMathLibrary.Lerp` 0.0 -100.0 _door_kick_track)) false false))))))
      (:`then_1`
        (`/Engine/EditorBlueprintResources/StandardMacros.DoOnce` true :!label _label
          (:`Completed`
            (`/Engine/EditorBlueprintResources/StandardMacros.Gate` true :!label _label_2
              (:`Exit`
                (`/Engine/EditorBlueprintResources/StandardMacros.FlipFlop`
                  (:`A`
                    (bind (_direction_2 _open_close_track) (`Timeline|Door Open T` :!via `ReverseFromEnd` :!label _label_3)
                      (:`Update`
                        (`SceneComponent.K2_SetRelativeRotation` (`self.Door`) (`KismetMathLibrary.MakeRotator` 0.0 0.0 (`KismetMathLibrary.Lerp` 0.0 -100.0 _open_close_track)) false false))))
                  (:`B`
                    (goto _label_3 :!via `PlayFromStart`))))))))))
  (:`Released`
    (goto _label :!via `Reset`)))

(event `self.Box.OnComponentBeginOverlap`
  (params (OverlappedComponent :type "PrimitiveComponent Object Reference") (OtherActor :type "Actor Object Reference") (OtherComp :type "PrimitiveComponent Object Reference") (OtherBodyIndex :type Integer) (bFromSweep :type Boolean) (SweepResult :type "HitResult Structure (by ref)"))
  (cast `/Game/ThirdPersonBP/Blueprints/ThirdPersonCharacter` OtherActor)
  (`self.EnableInput` (`GameplayStatics.GetPlayerController` 0))
  (goto _label_2 :!via `Open`))

(event `self.Box.OnComponentEndOverlap`
  (params (OverlappedComponent :type "PrimitiveComponent Object Reference") (OtherActor :type "Actor Object Reference") (OtherComp :type "PrimitiveComponent Object Reference") (OtherBodyIndex :type Integer))
  (cast `/Game/ThirdPersonBP/Blueprints/ThirdPersonCharacter` OtherActor)
  (`self.DisableInput` (`GameplayStatics.GetPlayerController` 0))
  (goto _label_2 :!via `Close`))

(fn `UserConstructionScript`)