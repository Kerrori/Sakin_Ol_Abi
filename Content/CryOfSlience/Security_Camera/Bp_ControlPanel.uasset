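; Security camera control panel that lets an interacting player view a set of security cameras.
; On interaction, if cameras exist and no one occupies it, it stores the player, moves input from player to panel and shows the first camera with a keyboard sound.
; Next and previous inputs cycle the camera index with wraparound, switching the PlayerController's view target.
; F returns view and input to the player and frees the panel.
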(event `/Game/CryOfSlience/Security_Camera/Interaction_Interface.OnInteraction`
  (params (Player :type "/Game/ThirdPersonBP/Blueprints/ThirdPersonCharacter Object Reference"))
  (bind _asplayer_controller (cast `PlayerController` (`Pawn.GetController` Player) :!pure true))
  (if (and (`self.HasCameras?`) (not (`self.Occupied?`)))
    (set `self.OccupiedPlayer` Player)
    (`self.DisableInput` Player _asplayer_controller)
    (`self.EnableInput` _asplayer_controller)
    (set `self.ActiveCameraIndex` 0)
    (`GameplayStatics.PlaySoundAtLocation` "/Game/CryOfSlience/Ses_Dosyası/keyboard_sound.keyboard_sound" (`self.K2_GetActorLocation`) (struct) 1.0 1.0 0.0 null null null)
    (`self.SetviewTargetAsActivaCamera`)))

(event `Key|F`
  (params (Key :type "Key Structure"))
  (bind _asplayer_controller (cast `PlayerController` (`Pawn.GetController` (`self.OccupiedPlayer`)) :!pure true))
  (:`Pressed`
    (`PlayerController.SetViewTargetWithBlend` _asplayer_controller (`self.OccupiedPlayer`) 0.0 "VTBlend_Linear" 0.0 false)
    (`self.EnableInput` (`self.OccupiedPlayer`) _asplayer_controller)
    (`self.DisableInput` _asplayer_controller)
    (set `self.OccupiedPlayer` null)))

(event `InputAction|Next Camera`
  (params (Key :type "Key Structure"))
  (:`Pressed`
    (`self.IncrementCameraIndex`)
    (`self.SetviewTargetAsActivaCamera`)))

(event `InputAction|PrevCamera`
  (params (Key :type "Key Structure"))
  (:`Pressed`
    (`self.DecrementCameraIndex`)
    (`self.SetviewTargetAsActivaCamera`)))

(fn `DecrementCameraIndex`
  (if (< (- (`self.ActiveCameraIndex`) 1) 0)
    (set `self.ActiveCameraIndex` (`KismetArrayLibrary.Array_LastIndex` (`self.SecurityCameras`)))
    (else
      (`/Engine/EditorBlueprintResources/StandardMacros.DecrementInt` (`self.ActiveCameraIndex`)))))

(fn `HasCameras?`
  (returns (ReturnValue :type Boolean))
  (return (> (`KismetArrayLibrary.Array_Length` (`self.SecurityCameras`)) 0)))

(fn `IncrementCameraIndex`
  (if (> (+ (`self.ActiveCameraIndex`) 1) (`KismetArrayLibrary.Array_LastIndex` (`self.SecurityCameras`)))
    (set `self.ActiveCameraIndex` 0)
    (else
      (`/Engine/EditorBlueprintResources/StandardMacros.IncrementInt` (`self.ActiveCameraIndex`)))))

(fn `Occupied?`
  (returns (ReturnValue :type Boolean))
  (return (`KismetSystemLibrary.IsValid` (`self.OccupiedPlayer`))))

(fn `SetviewTargetAsActivaCamera`
  (`PlayerController.SetViewTargetWithBlend` (cast `PlayerController` (`Pawn.GetController` (`self.OccupiedPlayer`)) :!pure true) (`|GetArrayItem` (`self.SecurityCameras`) (`self.ActiveCameraIndex`)) 0.0 "VTBlend_Linear" 0.0 false))

(fn `UserConstructionScript`)