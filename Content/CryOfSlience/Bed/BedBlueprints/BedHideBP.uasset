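; BedHideBP is a bed hiding spot that lets the player character toggle hiding with the Hide input.
; Box overlap stores the character, enables input and opens a gate, which closes on exit.
; Hiding blends the view to the bed, while a self-recalling short-delay loop applies clamped pitch and yaw to BedCamera.
; Look and turn input steers that camera when hidden, otherwise passes through to the character.
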(event `InputAction|Hide`
  (params (Key :type "Key Structure"))
  (bind _charref (`self.CharREF`))
  (:`Pressed`
    (`/Engine/EditorBlueprintResources/StandardMacros.Gate` true :!label _label
      (:`Exit`
        (if (`/Game/ThirdPersonBP/Blueprints/ThirdPersonCharacter.IsHiding?` _charref)
          (`/Game/ThirdPersonBP/Blueprints/ThirdPersonCharacter.Unhide` _charref)
          (else
            (`/Game/ThirdPersonBP/Blueprints/ThirdPersonCharacter.Hide` _charref)
            (`|ExecutionSequence`
              (:`then_0`
                (`PlayerController.SetViewTargetWithBlend` (`GameplayStatics.GetPlayerController` 0) self 0.5 "VTBlend_Linear" 0.0 false)
                (`self.Move Camera`))
              (:`then_1`
                (`KismetSystemLibrary.Delay` 0.2)
                (`self.EnableInput` (`GameplayStatics.GetPlayerController` 0) :!label _label_2)
                (goto _label :!via `Open`)))))))))

(event `self.Box.OnComponentBeginOverlap`
  (params (OverlappedComponent :type "PrimitiveComponent Object Reference") (OtherActor :type "Actor Object Reference") (OtherComp :type "PrimitiveComponent Object Reference") (OtherBodyIndex :type Integer) (bFromSweep :type Boolean) (SweepResult :type "HitResult Structure (by ref)"))
  (bind _asthird_person_character (cast `/Game/ThirdPersonBP/Blueprints/ThirdPersonCharacter` OtherActor))
  (set `self.CharREF` _asthird_person_character)
  (goto _label_2))

(event `self.Box.OnComponentEndOverlap`
  (params (OverlappedComponent :type "PrimitiveComponent Object Reference") (OtherActor :type "Actor Object Reference") (OtherComp :type "PrimitiveComponent Object Reference") (OtherBodyIndex :type Integer))
  (cast `/Game/ThirdPersonBP/Blueprints/ThirdPersonCharacter` OtherActor)
  (`self.DisableInput` (`GameplayStatics.GetPlayerController` 0))
  (goto _label :!via `Close`))

(event `Move Camera`
  (if (`/Game/ThirdPersonBP/Blueprints/ThirdPersonCharacter.IsHiding?` (`self.CharREF`))
    (`SceneComponent.K2_SetRelativeRotation` (`self.BedCamera`) (`KismetMathLibrary.MakeRotator` 0.0 (`KismetMathLibrary.FClamp` (* (stale `InputAxis|LookUp` _output_get) -1.0) -10.0 10.0) (`KismetMathLibrary.FClamp` (stale `InputAxis|Turn` _output_get) 60.0 120.0)) false false)
    (`KismetSystemLibrary.Delay` 0.001)
    (`self.Move Camera`)))

(event `InputAxis|LookUp`
  (params (AxisValue :type "Float (single-precision)"))
  (bind _charref (`self.CharREF`))
  (if (`/Game/ThirdPersonBP/Blueprints/ThirdPersonCharacter.IsHiding?` _charref)
    (bind _output_get (set `self.Pitch` (+ (`self.Pitch`) AxisValue)))
    (else
      (`Pawn.AddControllerPitchInput` _charref AxisValue))))

(event `InputAxis|Turn`
  (params (AxisValue :type "Float (single-precision)"))
  (bind _charref (`self.CharREF`))
  (if (`/Game/ThirdPersonBP/Blueprints/ThirdPersonCharacter.IsHiding?` _charref)
    (bind _output_get (set `self.Yaw` (+ (`self.Yaw`) AxisValue)))
    (else
      (`Pawn.AddControllerYawInput` _charref AxisValue))))

(fn `UserConstructionScript`)